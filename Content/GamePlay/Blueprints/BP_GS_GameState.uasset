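; Game State that runs a staged match of patrol, coin collection, sneak attack and team retreat, and scores each player.
; A timeline advances the stage enum, banks the previous stage's character scores and broadcasts the state change.
; Coins spawn in timed batches at random navmesh points and are destroyed afterward.
; Tick times the retreat as a negative team score for players still unscored, then Finish totals all four scores.
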(event `self.ReceiveBeginPlay`
  (`|ExecutionSequence`
    (:`then_0`
      (`self.SetPlayers`)
      (`self.StateChanged` "NewEnumerator11"))
    (:`then_1`
      (`Timeline|TL_StageScheduler`
        (:`Track`
          (`self.Manage Stage`))))))

(event `TossCoins`
  (`Timeline|TL_CoinScheduler`
    (:`EventTimes`
      (`self.SpawnCoins`))))

(event `self.ReceiveTick`
  (params (DeltaSeconds :type "Float (single-precision)"))
  (`self.CountTeamScore` DeltaSeconds))

(fn `CountTeamScore`
  (params (DeltaTime :type "Float (double-precision)"))
  (set `self.TeamTime` (+ DeltaTime (`self.TeamTime`))))

(fn `DestroyCoins`
  (bind _outactors (`GameplayStatics.GetAllActorsOfClass` "/Game/GamePlay/Blueprints/BP_A_Coin.BP_A_Coin_C"))
  (`self.K2_DestroyActor` _outactors))

(fn `GoToNextStage`
  (returns (Output_Get :type "/Game/GamePlay/Blueprints/E_Stage Enum"))
  (bind _output_get (set `self.Stage` (cast `/Game/GamePlay/Blueprints/E_Stage` (+ (`self.Stage`) 1))))
  (return _output_get))

(fn `Manage Stage`
  (bind _output_get (`self.GoToNextStage`))
  (`|ExecutionSequence`
    (:`then_0`
      (switch `/Game/GamePlay/Blueprints/E_Stage` _output_get
        (:`NewEnumerator19`
          (`self.SetPatrolScore`)
          (`self.TossCoins`))
        (:`NewEnumerator23`
          (`self.SetCoinScore`)
          (`self.DestroyCoins`))
        (:`NewEnumerator27`
          (`self.SetSneakScore`)
          (`self.SetActorTickEnabled` true))
        (:`NewEnumerator28`
          (`self.SetTeamsScore`)
          (`self.SetSumScore`))))
    (:`then_1`
      (`self.StateChanged` _output_get))))

(fn `SetCoinScore`
  (for _array_element (`self.Players`)
    (`KismetArrayLibrary.Array_Set` (`self.CoinScore`) (break `/Game/GamePlay/Blueprints/S_Player` _array_element) (`KismetMathLibrary.Round` (`|GetArrayItem` (`/Game/GamePlay/Blueprints/AI_Character.Score` (`.Character_11_915A078A42B771167CC51598790362E1` (break `/Game/GamePlay/Blueprints/S_Player` _array_element))) 1)))))

(fn `SetPatrolScore`
  (for _array_element (`self.Players`)
    (`KismetArrayLibrary.Array_Set` (`self.PatrolScore`) (break `/Game/GamePlay/Blueprints/S_Player` _array_element) (`KismetMathLibrary.Round` (/ (`|GetArrayItem` (`/Game/GamePlay/Blueprints/AI_Character.Score` (`.Character_11_915A078A42B771167CC51598790362E1` (break `/Game/GamePlay/Blueprints/S_Player` _array_element)))) 1000.0)))))

(fn `SetPlayers`
  (bind _asbp_gm_game_mode (cast `/Game/GamePlay/Blueprints/BP_GM_GameMode` (`GameplayStatics.GetGameMode`)))
  (set `self.Players` (`/Game/GamePlay/Blueprints/BP_GM_GameMode.Players` _asbp_gm_game_mode)))

(fn `SetSneakScore`
  (for _array_element (`self.Players`)
    (`KismetArrayLibrary.Array_Set` (`self.SneakScore`) (break `/Game/GamePlay/Blueprints/S_Player` _array_element) (`KismetMathLibrary.Round` (`|GetArrayItem` (`/Game/GamePlay/Blueprints/AI_Character.Score` (`.Character_11_915A078A42B771167CC51598790362E1` (break `/Game/GamePlay/Blueprints/S_Player` _array_element))) 2)))))

(fn `SetSumScore`
  (locals (NewLocalVar_0 :type Boolean))
  (for _array_element (`self.Players`)
    (`KismetArrayLibrary.Array_Set` (`self.Score`) (break `/Game/GamePlay/Blueprints/S_Player` _array_element) (+ (`|GetArrayItem` (`self.TeamScore`) (break `/Game/GamePlay/Blueprints/S_Player` _array_element)) (`|GetArrayItem` (`self.SneakScore`) (break `/Game/GamePlay/Blueprints/S_Player` _array_element)) (`|GetArrayItem` (`self.CoinScore`) (break `/Game/GamePlay/Blueprints/S_Player` _array_element)) (`|GetArrayItem` (`self.PatrolScore`) (break `/Game/GamePlay/Blueprints/S_Player` _array_element))))))

(fn `SetTeamScore`
  (params (`Team Index` :type Integer))
  (locals (NewLocalVar_0 :type Boolean))
  (for _array_element (`self.Players`)
    (if (and (== (`|GetArrayItem` (`self.TeamScore`) (break `/Game/GamePlay/Blueprints/S_Player` _array_element)) 0) (== (`.Team_5_C89400B34FD76B48FC6815AFCB46DE53` (break `/Game/GamePlay/Blueprints/S_Player` _array_element)) `Team Index`))
      (`KismetArrayLibrary.Array_Set` (`self.TeamScore`) (break `/Game/GamePlay/Blueprints/S_Player` _array_element) (`KismetMathLibrary.FTrunc` (* -1 (`self.TeamTime`)))))))

(fn `SetTeamsScore`
  (locals (NewLocalVar_0 :type Boolean))
  (`self.SetActorTickEnabled` false)
  (for _index (range 3)
    (`self.SetTeamScore` _index)))

(fn `SpawnCoins`
  (for _ (range 10)
    (`|SpawnActorFromClass` "/Game/GamePlay/Blueprints/BP_A_Coin.BP_A_Coin_C" (`KismetMathLibrary.Conv_VectorToTransform` (`NavigationSystemV1.K2_GetRandomReachablePointInRadius` (0.0 0.0 180.0) 1100.0 null null)) "Undefined" "OverrideRootScale" null null)))

(fn `UserConstructionScript`)